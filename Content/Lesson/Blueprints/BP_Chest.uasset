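; BP_Chest is an interactable chest with two key slots that spends the player's keys to open.
; Each Interact call, while closed, takes one key from BP_Player if available and branches on KeysLeft.
; Timelines slide and spin the revealed key mesh into its slot.
; The last key sets IsOpen immediately, and its finished animation chains into a second timeline that rotates the lid open.
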(event EventInteract
  (bind _returnvalue (Game|GetPlayerCharacter 0))
  (bind _returnvalue_2 (Game|GetPlayerCharacter 0))
  (bind _asbp_player (Utilities|Casting|CastToBP_Player _returnvalue))
  (bind _asbp_player_2 (Utilities|Casting|CastToBP_Player _returnvalue_2))
  (bind _nbkeys (Variables|/Game/Lesson/Blueprints/BP_Player.BP_Player_C|GetNbKeys _asbp_player))
  (bind _nbkeys_2 (Variables|/Game/Lesson/Blueprints/BP_Player.BP_Player_C|GetNbKeys _asbp_player_2))
  (if (not (Variables|Default|GetIsOpen))
    (switch int (Variables|Default|GetKeysLeft)
      (:1
        (if (> _nbkeys 0)
          (Variables|Default|SetIsOpen true)
          (Math|Integer|DecrementInt _nbkeys
            (:%20%20
              (Math|Integer|DecrementInt (Variables|Default|GetKeysLeft)
                (:%20%20
                  (Rendering|SetVisibility (Variables|Default|GetSM_Key2) true false)
                  (bind (_direction _location _rotation) (Timeline|Timeline Play)
                    (:Update
                      (Transformation|SetRelativeLocation (Variables|Default|GetSM_Key2) (Math|Vector|Lerp(Vector) "19.000000,104.000000,6.000000" "19.000000,84.000000,6.000000" _location) false false)
                      (Transformation|SetRelativeRotation (Variables|Default|GetSM_Key2) (Math|Rotator|Lerp(Rotator) "0.000000,-90.000000,-90.000000" "0.000000,-90.000000,-450.000000" _rotation) false false))
                    (:Finished
                      (bind _location_2 (Timeline|Timeline_0 Play)
                        (:Update
                          (Transformation|SetRelativeRotation (Variables|Default|GetChest_cover6_StaticMeshComponent0) (Math|Rotator|MakeRotator (* _location_2 -6e+01) 0.0 0.0) false false)))))))))))
      (:2
        (if (> _nbkeys_2 0)
          (Math|Integer|DecrementInt _nbkeys_2
            (:%20%20
              (Math|Integer|DecrementInt (Variables|Default|GetKeysLeft)
                (:%20%20
                  (Rendering|SetVisibility (Variables|Default|GetSM_Key1) true false)
                  (bind (_direction_2 _location_3 _rotation_2) (Timeline|MoveKey1 Play)
                    (:Update
                      (Transformation|SetRelativeLocation (Variables|Default|GetSM_Key1) (Math|Vector|Lerp(Vector) "-19.000000,104.000000,6.000000" "-19.000000,84.000000,6.000000" _location_3) false false)
                      (Transformation|SetRelativeRotation (Variables|Default|GetSM_Key1) (Math|Rotator|Lerp(Rotator) "0.000000,-90.000000,-90.000000" "0.000000,-90.000000,-450.000000" _rotation_2) false false))))))))))))

(fn ConstructionScript)